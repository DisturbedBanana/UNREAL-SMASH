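; BP_Character_Jammus is the Blueprint for Jammus, a character in SmashUE with a StateMachine.
; Its event graph holds leftover logic for switching between Idle, Walk and Run, including checks on the current state with debug prints when Idle.
; None of these fragments is wired to an event, so they never run, and the construction script is empty.
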(fn `UserConstructionScript`)